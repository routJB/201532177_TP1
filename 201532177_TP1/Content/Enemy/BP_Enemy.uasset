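; BP_Enemy is a flipbook-sprite demon (Pinky) that hunts and attacks the first-person player and dies from any damage.
; PawnSensing sighting starts an AIMoveTo toward the player and enables per-tick yaw rotation to face them.
; Reaching the player triggers the attack animation, sound and a sphere-overlap damage check around AttackSphere.
; Any damage stops movement and plays death sound and flipbooks before destroying the actor.
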(event `self.ReceiveTick`
  (params (DeltaSeconds :type "Float (single-precision)"))
  (bind (_returnvalue_roll _returnvalue_pitch _returnvalue_yaw) (`KismetMathLibrary.BreakRotator` (`KismetMathLibrary.FindLookAtRotation` (`self.K2_GetActorLocation`) (`self.K2_GetActorLocation` (`GameplayStatics.GetPlayerCharacter` 0)))))
  ;[1 1 1] Faire face au joueur
  (if (`self.peutvoirjoueur`)
    (`self.K2_SetActorRotation` (`KismetMathLibrary.MakeRotator` 0.0 0.0 _returnvalue_yaw))))

(event `self.PawnSensing.OnSeePawn`
  (params (Pawn :type "Pawn Object Reference"))
  ;[1 1 1] Déplacement et attaque
  (bind _asbp_first_person_character (cast `/Game/FirstPerson/Blueprints/BP_FirstPersonCharacter` Pawn))
  (set `self.peutvoirjoueur` true)
  (`|AIMoveTo` self (0.0 0.0 0.0) _asbp_first_person_character
    (:`OnSuccess`
      (`self.Attack`))
    (:`OnFail`
      (`PaperFlipbookComponent.SetFlipbook` (`self.PaperFlipbook`) "/Game/Enemy/PinkyMove.PinkyMove"))))

(event `self.ReceiveAnyDamage`
  (params (Damage :type "Float (single-precision)") (DamageType :type "DamageType Object Reference") (InstigatedBy :type "Controller Object Reference") (DamageCauser :type "Actor Object Reference"))
  (bind _paperflipbook (`self.PaperFlipbook`))
  ;[1 1 1] Prendre des dégats
  (`ActorComponent.Deactivate` (`self.CharacterMovement`))
  (`GameplayStatics.PlaySound2D` "/Game/Sounds/Demons/demon_death.demon_death" 1.0 1.0 0.0 null null)
  (`PaperFlipbookComponent.SetFlipbook` _paperflipbook "/Game/Enemy/pinkydeath.pinkydeath")
  (`KismetSystemLibrary.Delay` (`PaperFlipbookComponent.GetFlipbookLength` _paperflipbook))
  (`PaperFlipbookComponent.SetFlipbook` (`self.PaperFlipbook`) "/Game/Enemy/deadpinky.deadpinky")
  (`KismetSystemLibrary.Delay` 0.2)
  (`self.K2_DestroyActor` self))

(event `Attack`
  (`PaperFlipbookComponent.SetFlipbook` (`self.PaperFlipbook`) "/Game/Enemy/pinkyattack.pinkyattack")
  (`self.Deal Damage`)
  (`GameplayStatics.PlaySound2D` "/Game/Sounds/Demons/demon_attack.demon_attack" 1.0 1.0 0.0 null null))

(event `Deal Damage`
  ;[1 1 1] DealDamage
  (bind _outactors (`KismetSystemLibrary.SphereOverlapActors` (`SceneComponent.K2_GetComponentLocation` (`self.Attack Sphere`)) 50.0 (`|MakeArray` "ObjectTypeQuery3" :!type "EObjectTypeQuery Enum") "/Game/FirstPerson/Blueprints/BP_FirstPersonCharacter.BP_FirstPersonCharacter_C" (`|MakeArray` self :!type "Actor Object Reference")))
  (for _array_element _outactors
    (`GameplayStatics.ApplyDamage` _array_element (`self.Base damage`) (`self.GetController`) self "/Script/Engine.DamageType")))

(fn `UserConstructionScript`)