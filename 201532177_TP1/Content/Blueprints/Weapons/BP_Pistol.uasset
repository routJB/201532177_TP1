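; Pistol weapon Blueprint that handles firing and its 2D flipbook animation.
; ShootWeapon passes through a DoOnce, calls Fireweapon (defined outside this file) and switches the Paper2D flipbook to the fire animation.
; After a delay equal to that flipbook's length, it restores the idle flipbook and calls Resetweapon to reopen the DoOnce, so fire rate follows animation length.
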(event `self.ShootWeapon`
  (bind _weaponflipbook (`self.Weaponflipbook`))
  (`/Engine/EditorBlueprintResources/StandardMacros.DoOnce` false :!label _label
    (:`Completed`
      (`self.Fireweapon`)
      (`PaperFlipbookComponent.SetFlipbook` _weaponflipbook "/Game/Sprites/Weapons/Pistol/pistolfire.pistolfire")
      (`KismetSystemLibrary.Delay` (`PaperFlipbookComponent.GetFlipbookLength` _weaponflipbook))
      (`PaperFlipbookComponent.SetFlipbook` (`self.Weaponflipbook`) "/Game/Sprites/Weapons/Pistol/pistolidle.pistolidle")
      (`self.Resetweapon`))))

(event `Resetweapon`
  (goto _label :!via `Reset`))

(fn `UserConstructionScript`
  (`parent.UserConstructionScript`))